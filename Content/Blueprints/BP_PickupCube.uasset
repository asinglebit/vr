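; Pickup cube that a motion controller can grab and drop by attachment, physics handle or a mixed mode.
; Pickup and drop events dispatch on the selected grab method and track the holding controller and handle.
; In mixed mode, Tick switches the attached cube to the physics handle when it overlaps other objects.
; Once clear, it lerps back to its stored controller-relative offset and reattaches, with resettable DoOnce gates guarding each switch.
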(event Custom|OpenDoOnceGates
  (Utilities|FlowControl|Sequence
    (:then_0
      (Utilities|FlowControl|DoOnce false) ; enters at Reset
    )
    (:then_1
      (Utilities|FlowControl|DoOnce false) ; enters at Reset
    )))

(event EventTick
  (params (DeltaSeconds :type Float%20%28single-precision%29))
  (bind _staticmeshcomponent (Variables|Default|GetStaticMeshComponent))
  (switch Utilities|FlowControl|Switch|SwitchonEnumGrabMethod (Variables|Default|GetEGrabMethod)
    (:PhysicalHandle
      (Class|PickupStaticMeshActor|FDropifLostConnection))
    (:Mixed
      (Class|PickupStaticMeshActor|FDropifLostConnection)
      (if (Utilities|IsValid (Variables|Default|GetAMotionController))
        (bind _returnvalue (Class|KismetSystemLibrary|ComponentOverlapComponents _staticmeshcomponent (Transformation|GetWorldTransform _staticmeshcomponent) (Utilities|Array|MakeArray "ObjectTypeQuery1" "ObjectTypeQuery2" "ObjectTypeQuery4" "ObjectTypeQuery7") 0 (Variables|Default|GetAActorsToIgnore)))
        (if _returnvalue
          (Utilities|FlowControl|DoOnce false :!label _label
            (:Completed
              (Class|PickupStaticMeshActor|FDropAttachto)
              (CallFunction|GrabPhysicsHandle)
              (goto _label_2 Reset)))
          (elif (not (< (- (Utilities|Time|GetGameTimeinSeconds) (Variables|Default|GetFHitTime)) 0.1))
            (if (> (Variables|Default|GetFLocationAlpha) 1.0)
              (Utilities|FlowControl|DoOnce false :!label _label_2
                (:Completed
                  (Class|PickupStaticMeshActor|FDropPhysicsHandle)
                  (CallFunction|GrabAttachto)
                  (goto _label Reset)))
              (else
                (Variables|Default|SetFLocationAlpha (+ (Variables|Default|GetFLocationAlpha) (* (Utilities|Time|GetWorldDeltaSeconds) 1e+01)))
                (Transformation|SetWorldLocationAndRotation (Variables|Default|GetStaticMeshComponent) (.location (Math|Transform|Lerp(Transform) (Transformation|GetWorldTransform (Variables|Default|GetStaticMeshComponent)) (Utilities|GetWorldPickupTransform) (Variables|Default|GetFLocationAlpha))) (.rotation (Math|Transform|Lerp(Transform) (Transformation|GetWorldTransform (Variables|Default|GetStaticMeshComponent)) (Utilities|GetWorldPickupTransform) (Variables|Default|GetFLocationAlpha))) false false)))))))))

(event EventFPickup
  (params (MotionController :type Scene%20Component%20Object%20Reference) (PhysicsHandler :type Physics%20Handle%20Component%20Object%20Reference))
  (Utilities|FlowControl|Sequence
    (:then_0
      (Utilities|IsValid (Variables|Default|GetAMotionController)
        (:Is%20Valid
          (Class|PickupActor|FDrop))))
    (:then_1
      (Variables|Default|SetAMotionController MotionController)
      (Variables|Default|SetAPhysicsHandle PhysicsHandler))
    (:then_2
      (switch Utilities|FlowControl|Switch|SwitchonEnumGrabMethod (Variables|Default|GetEGrabMethod)
        (:AttachedTo
          (CallFunction|GrabAttachto))
        (:PhysicalHandle
          (CallFunction|GrabPhysicsHandle))
        (:Mixed
          (CallFunction|GrabMixedMode))))))

(event EventFDrop
  (Utilities|FlowControl|Sequence
    (:then_0
      (switch Utilities|FlowControl|Switch|SwitchonEnumGrabMethod (Variables|Default|GetEGrabMethod)
        (:AttachedTo
          (Class|PickupStaticMeshActor|FDropAttachto))
        (:PhysicalHandle
          (Class|PickupStaticMeshActor|FDropPhysicsHandle))
        (:Mixed
          (CallFunction|DropMixedMode))))
    (:then_1
      (Variables|Default|SetAMotionController 0)
      (Variables|Default|SetAPhysicsHandle 0))))

(fn ConstructionScript)

(fn GrabAttachto
  (bind _transform (Utilities|GetWorldPickupTransform))
  (Collision|SetCollisionObjectType (Variables|Default|GetStaticMeshComponent) "ECC_GameTraceChannel2")
  (Physics|SetEnableGravity (Variables|Default|GetStaticMeshComponent) false)
  (Physics|SetSimulatePhysics (Variables|Default|GetStaticMeshComponent) false)
  (if (Variables|Default|GetBIsMixedModeGrabbed)
    (Transformation|SetWorldLocationAndRotation (Variables|Default|GetStaticMeshComponent) (.location _transform) (.rotation _transform) false false))
  (Transformation|AttachComponentToComponent (VehicleSound|GetRootComponent) (Variables|Default|GetAMotionController) "None" "KeepWorld" "KeepWorld" "KeepWorld" false)
  (if (not (Variables|Default|GetBIsMixedModeGrabbed))
    (Variables|Default|SetTRelativePickupOffset (Utilities|GetRelativePickupTransform))))

(fn GrabPhysicsHandle
  (bind _amotioncontroller (Variables|Default|GetAMotionController))
  (bind _returnvalue (Transformation|GetWorldTransform _amotioncontroller))
  (Physics|Components|PhysicsHandle|GrabComponentatLocationwithRotation (Variables|Default|GetAPhysicsHandle) (Variables|Default|GetStaticMeshComponent) "None" (.location _returnvalue) (.rotation _returnvalue))
  (Physics|SetEnableGravity (Variables|Default|GetStaticMeshComponent) false)
  (Physics|SetSimulatePhysics (Variables|Default|GetStaticMeshComponent) true)
  (Collision|SetCollisionObjectType (Variables|Default|GetStaticMeshComponent) "ECC_PhysicsBody")
  (Variables|Default|SetFLocationAlpha 0.0))

(fn GrabMixedMode
  (Collision|SetCollisionResponsetoChannel (Variables|Default|GetStaticMeshComponent) "ECC_Pawn" "ECR_Ignore")
  (CallFunction|GrabAttachto)
  (Variables|Default|SetBIsMixedModeGrabbed true)
  (CallFunction|OpenDoOnceGates))

(fn DropMixedMode
  (Variables|Default|SetBIsMixedModeGrabbed false)
  (Class|PickupStaticMeshActor|FDropPhysicsHandle)
  (Class|PickupStaticMeshActor|FDropAttachto)
  (Collision|SetCollisionObjectType (Variables|Default|GetStaticMeshComponent) "ECC_PhysicsBody")
  (Collision|SetCollisionResponsetoChannel (Variables|Default|GetStaticMeshComponent) "ECC_Pawn" "ECR_Block")
  (Variables|Default|SetFLocationAlpha 0.0))

(fn FIsHeldbyMe
  (params (MotionController :type Scene%20Component%20Object%20Reference))
  (return (== MotionController (Variables|Default|GetAMotionController))))